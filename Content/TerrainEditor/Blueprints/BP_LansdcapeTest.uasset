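; Terrain editor actor that procedurally generates a Landscape's heightmap from a noise material.
; The construction script builds a dynamic instance of MI_TerrainConstructor from three Perlin layers, Voronoi and overall height settings, redrawing when HotCookLandscape is on.
; DrawToRT renders that material to a render target and imports it as the Landscape heightmap.
; RandomizeTerrainLocation shifts the world-aligned noise by a random offset, then redraws.
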(event `DrawToRT`
  ;[1 1 1] Update Heightmap Render Target, apply Heightmap RT to Landscape, updating geometry/collisions
  (`KismetRenderingLibrary.DrawMaterialToRenderTarget` null (`self.RT`) (`self.TerrainMat`))
  (`LandscapeProxy.LandscapeImportHeightmapFromRenderTarget` (`self.Landscape`) (`self.RT`) false))

(event `RandomizeTerrainLocation`
  ;[1 1 1] Apply random location offset to world-aligned noise textures generated for heightmap, updates landscape when called
  (set `self.RandomOffset` (`KismetMathLibrary.RandomFloatInRange` -5000000.0 5000000.0))
  (`MaterialInstanceDynamic.SetScalarParameterValue` (`self.TerrainMat`) "RandomOffset" (`self.RandomOffset`))
  (`self.DrawToRT`))

(fn `Assign Variables to Terrain Construction Dynamic Material`
  (bind _terrainmat (`self.TerrainMat`))
  (bind _returnvalue (`KismetMaterialLibrary.CreateDynamicMaterialInstance` null "/Game/TerrainEditor/Materials/Instances/MI_TerrainConstructor.MI_TerrainConstructor"))
  (bind _output_get (set `self.TerrainMat` _returnvalue))
  (`MaterialInstanceDynamic.SetScalarParameterValue` _output_get "PerlinScale1" (`self.PerlinScale1`))
  (`MaterialInstanceDynamic.SetScalarParameterValue` _output_get "PerlinContrast1" (`self.PerlinContrast1`))
  (`MaterialInstanceDynamic.SetScalarParameterValue` _output_get "PerlinStrength1" (`self.PerlinStrength1`))
  (`MaterialInstanceDynamic.SetScalarParameterValue` _output_get "Perlin1" (`self.Perlin1`))
  (`MaterialInstanceDynamic.SetScalarParameterValue` _output_get "PerlinScale2" (`self.PerlinScale2`))
  (`MaterialInstanceDynamic.SetScalarParameterValue` _output_get "PerlinContrast2" (`self.PerlinContrast2`))
  (`MaterialInstanceDynamic.SetScalarParameterValue` _output_get "PerlinStrength2" (`self.PerlinStrength2`))
  (`MaterialInstanceDynamic.SetScalarParameterValue` _output_get "Perlin2" (`self.Perlin2`))
  (`MaterialInstanceDynamic.SetScalarParameterValue` _output_get "PerlinScale3" (`self.PerlinScale3`))
  (`MaterialInstanceDynamic.SetScalarParameterValue` _output_get "PerlinContrast3" (`self.PerlinContrast3`))
  (`MaterialInstanceDynamic.SetScalarParameterValue` _output_get "PerlinStrength3" (`self.PerlinStrength3`))
  (`MaterialInstanceDynamic.SetScalarParameterValue` _output_get "Perlin3" (`self.Perlin3`))
  (`MaterialInstanceDynamic.SetScalarParameterValue` (`self.TerrainMat`) "OverallHeight" (`self.OverallHeight`))
  (`MaterialInstanceDynamic.SetScalarParameterValue` _terrainmat "VoronoiContrast" (`self.VoronoiContrast`))
  (`MaterialInstanceDynamic.SetScalarParameterValue` _terrainmat "VoronoiStrength" (`self.VoronoiStrength`))
  (`MaterialInstanceDynamic.SetScalarParameterValue` _terrainmat "VoronoiScale" (`self.VoronoiScale`))
  (`MaterialInstanceDynamic.SetScalarParameterValue` _terrainmat "Voronoi" (`self.Voronoi`))
  (`MaterialInstanceDynamic.SetScalarParameterValue` _terrainmat "VoronoiBreakup" (`self.VoronoiBreakup`))
  (return))

(fn `UserConstructionScript`
  (`self.Assign Variables to Terrain Construction Dynamic Material`)
  (if (`self.HotCookLandscape`)
    (`self.DrawToRT`)))